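; BP_Player is the player Blueprint that routes input for camera, movement and shooting.
; Axis inputs pass their values to camera and movement functions, and actions call crouch, sprint, roll, fire and aim functions.
; Only fire and aim respond to both press and release; crouch, sprint and roll respond to press only.
; The called functions are defined outside these graphs, and the construction script is empty.
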(event `InputAxis|Mouse Pitch`
  (params (AxisValue :type "Float (single-precision)"))
  ;[1 1 1] Camera Movement
  (`self.MoveCameraVertical` AxisValue))

(event `InputAction|Crouch`
  (params (Key :type "Key Structure"))
  ;[1 1 1] Movement
  (:`Pressed`
    (`self.Crouching`)))

(event `InputAxis|Vertical`
  (params (AxisValue :type "Float (single-precision)"))
  ;[1 1 1] Movement
  (`self.MoveForward` AxisValue))

(event `InputAxis|Mouse Yaw`
  (params (AxisValue :type "Float (single-precision)"))
  ;[1 1 1] Camera Movement
  (`self.MoveCameraHorizontal` AxisValue))

(event `InputAction|Shoot`
  (params (Key :type "Key Structure"))
  ;[1 1 1] Shooting
  (:`Pressed`
    (`self.StartFire`))
  (:`Released`
    (`self.StopFire`)))

(event `InputAction|Sprint`
  (params (Key :type "Key Structure"))
  ;[1 1 1] Movement
  (:`Pressed`
    (`self.StartSprint`)))

(event `InputAxis|Horizontal`
  (params (AxisValue :type "Float (single-precision)"))
  ;[1 1 1] Movement
  (`self.MoveHorizontal` AxisValue))

(event `InputAction|Roll`
  (params (Key :type "Key Structure"))
  ;[1 1 1] Movement
  (:`Pressed`
    (`self.Rolling`)))

(event `InputAction|Aim`
  (params (Key :type "Key Structure"))
  ;[1 1 1] Camera Movement
  (:`Pressed`
    (`self.StartAim`))
  (:`Released`
    (`self.StopAim`)))

(fn `UserConstructionScript`)
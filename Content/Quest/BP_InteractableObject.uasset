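; Quest interactable actor that adds to a quest counter when the player interacts with it.
; Overlapping its collision calls InteractWithPlayer, shows a HUD pop-up and binds OnInteract to the player's interact dispatcher.
; On interaction, it adds ValueToAdd under its ID through the controller's QuestComponent, destroys itself and hides the pop-up.
; Ending overlap hides the pop-up and unbinds all events from that dispatcher.
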(event `self.CollisionComponent.OnComponentBeginOverlap`
  (params (OverlappedComponent :type "PrimitiveComponent Object Reference") (OtherActor :type "Actor Object Reference") (OtherComp :type "PrimitiveComponent Object Reference") (OtherBodyIndex :type Integer) (bFromSweep :type Boolean) (SweepResult :type "HitResult Structure (by ref)"))
  (`self.InteractWithPlayer` true OtherActor)
  (bind _asbp_hud (cast `/Game/UI/BP_HUD` (`PlayerController.GetHUD` (`GameplayStatics.GetPlayerController` 0))))
  (`/Game/UI/BP_HUD.ActivatePopUp` _asbp_hud "Visible")
  (bind _asbp_player (cast `/Game/Player/BP_Player` (`GameplayStatics.GetPlayerCharacter` 0)))
  (add `/Game/Player/BP_Player.OnInteract` _asbp_player (delegate `OnInteract`)))

(event `OnInteract`
  (`QuestComponent.AddCounter` (`self.GetComponentByClass` (`GameplayStatics.GetPlayerController` 0) "/Script/UnrealEndYearProject.QuestComponent") (`self.ID`) (`self.Value to Add`))
  (`self.K2_DestroyActor`)
  (bind _asbp_hud (cast `/Game/UI/BP_HUD` (`PlayerController.GetHUD` (`GameplayStatics.GetPlayerController` 0))))
  (`/Game/UI/BP_HUD.ActivatePopUp` _asbp_hud "Hidden")
  (clear `/Game/Player/BP_Player.OnInteract` (stale `self.CollisionComponent.OnComponentBeginOverlap` _asbp_player)))

(event `self.CollisionComponent.OnComponentEndOverlap`
  (params (OverlappedComponent :type "PrimitiveComponent Object Reference") (OtherActor :type "Actor Object Reference") (OtherComp :type "PrimitiveComponent Object Reference") (OtherBodyIndex :type Integer))
  (`self.InteractWithPlayer` false OtherActor)
  (bind _asbp_hud (cast `/Game/UI/BP_HUD` (`PlayerController.GetHUD` (`GameplayStatics.GetPlayerController` 0))))
  (`/Game/UI/BP_HUD.ActivatePopUp` _asbp_hud "Hidden")
  (bind _asbp_player (cast `/Game/Player/BP_Player` (`GameplayStatics.GetPlayerCharacter` 0)))
  (clear `/Game/Player/BP_Player.OnInteract` _asbp_player))

(fn `UserConstructionScript`)